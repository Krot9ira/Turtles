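; NestButtonBP is a pressable button that spawns turtles from a nest.
; A box overlap registers it as the current Button on TempPawnBP and clears it on exit.
; SpawnTurtles briefly sinks the button mesh while sending SpawnTurtleMessage with BTType to its Target, then sets AlreadySpawned.
; The one-spawn-per-button check on that flag is left unwired, so spawns are unlimited.
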(event `SpawnTurtles`
  (`SceneComponent.K2_SetRelativeLocation` (`self.Buttonmain`) (0.0 0.0 -5.0) false false)
  (message `/Game/Blueprints/Interfaces/NestInterface.SpawnTurtle` (`self.Target`) (`self.BTType`))
  (`KismetSystemLibrary.Delay` 0.2)
  (`SceneComponent.K2_SetRelativeLocation` (`self.Buttonmain`) (0.0 0.0 0.0) false false)
  (set `self.AlreadySpawned` true))

(event `self.Box.OnComponentBeginOverlap`
  (params (OverlappedComponent :type "PrimitiveComponent Object Reference") (OtherActor :type "Actor Object Reference") (OtherComp :type "PrimitiveComponent Object Reference") (OtherBodyIndex :type Integer) (bFromSweep :type Boolean) (SweepResult :type "HitResult Structure (by ref)"))
  (bind _astemp_pawn_bp (cast `/Game/Blueprints/TempPawn/TempPawnBP` OtherActor))
  (set `/Game/Blueprints/TempPawn/TempPawnBP.Button` self _astemp_pawn_bp))

(event `self.Box.OnComponentEndOverlap`
  (params (OverlappedComponent :type "PrimitiveComponent Object Reference") (OtherActor :type "Actor Object Reference") (OtherComp :type "PrimitiveComponent Object Reference") (OtherBodyIndex :type Integer))
  (bind _astemp_pawn_bp (cast `/Game/Blueprints/TempPawn/TempPawnBP` OtherActor))
  (set `/Game/Blueprints/TempPawn/TempPawnBP.Button` null _astemp_pawn_bp))

(fn `UserConstructionScript`)