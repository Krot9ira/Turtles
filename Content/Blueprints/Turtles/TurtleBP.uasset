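; TurtleBP is a turtle actor that handles its own spawn burst, walk sound and attached aura effect.
; BeginPlay stores the home position, attaches the walk sound and heal-aura particles, and spawns an aqua storm burst below the capsule that is destroyed after a short delay.
; A Stop event halts the sound, clears the playing flag and destroys the aura.
; No movement logic lives in this graph.
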(event `self.ReceiveBeginPlay`
  (bind (_returnvalue_x _returnvalue_y _returnvalue_z) (`KismetMathLibrary.BreakVector` (`SceneComponent.K2_GetComponentLocation` (`self.CapsuleComponent`))))
  (set `self.HomePosition` (`SceneComponent.K2_GetComponentLocation` (`self.CapsuleComponent`)))
  (bind _returnvalue (`GameplayStatics.SpawnSoundAttached` (`self.WalkSound`) (`self.CapsuleComponent`) "None" (0.0 0.0 0.0) (struct) "KeepRelativeOffset" false 1.0 1.0 0.0 null null))
  (set `self.WalkSoundRef` _returnvalue)
  (set `self.IsPlaying` true)
  (bind _returnvalue_2 (`GameplayStatics.SpawnEmitterAtLocation` "/Game/FXVarietyPack/Particles/P_ky_aquaStorm.P_ky_aquaStorm" (`KismetMathLibrary.MakeVector` _returnvalue_x _returnvalue_y (- _returnvalue_z 50.0)) (struct) (0.5 0.5 0.5)))
  (bind _returnvalue_3 (`GameplayStatics.SpawnEmitterAttached` "/Game/FXVarietyPack/Particles/P_ky_healAura.P_ky_healAura" (`self.Scene`) "None" (0.0 0.0 0.0) (struct) (1.0 1.0 1.0) "KeepRelativeOffset" false))
  (set `self.WalkEffect` _returnvalue_3)
  (`KismetSystemLibrary.Delay` 3.0)
  (`ActorComponent.K2_DestroyComponent` _returnvalue_2))

(event `self.ReceiveTick`
  (params (DeltaSeconds :type "Float (single-precision)")))

(event `Stop`
  (`AudioComponent.Stop` (`self.WalkSoundRef`))
  (set `self.IsPlaying` false)
  (`ActorComponent.K2_DestroyComponent` (`self.WalkEffect`)))

(fn `UserConstructionScript`)